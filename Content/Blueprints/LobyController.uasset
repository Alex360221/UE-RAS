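; LobyController is a lobby actor Blueprint for starting multiplayer games and moving to game maps.
; StartGameServer opens AnotherRopeTEstingLevel as a listen server, while StartGameClient is an empty stub.
; StartGame issues a servertravel console command toward RAS_Testing, appended without a separating space; both IP inputs go unused.
; The remaining StartGame logic is unreachable debug and test code for controller printing, rope spawning and level opening.
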(event Custom|StartGameServer
  (params (IP :type Name))
  (Game|OpenLevel(byName) "AnotherRopeTEstingLevel" true "listen"))

(event Custom|StartGameClient)

(event EventBeginPlay)

(event Collision|EventActorBeginOverlap
  (params (OtherActor :type Actor%20Object%20Reference)))

(event EventTick
  (params (DeltaSeconds :type Float%20%28single-precision%29)))

(fn ConstructionScript)

(fn StartGame
  (params (IP :type Name))
  (Development|ExecuteConsoleCommand (Utilities|String|Append "servertravel " "RAS_Testing") 0))