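; Teleport actor that moves a standard or VR player character from its trigger box to the location of a linked OtherEnd actor.
; Box overlap events set InBox and store the overlapping Character as Player.
; While InBox is set, Tick polls that character's MoveUp flag, teleports it without sweep, then clears the flag.
; Any other stored character type clears InBox.
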(event OnComponentBeginOverlap(Box)
  (params (OverlappedComponent :type Primitive%20Component%20Object%20Reference) (OtherActor :type Actor%20Object%20Reference) (OtherComp :type Primitive%20Component%20Object%20Reference) (OtherBodyIndex :type Integer) (bFromSweep :type Boolean) (SweepResult :type Hit%20Result%20Structure%20%28by%20ref%29))
  (Variables|Default|SetInBox true)
  (bind _ascharacter (Utilities|Casting|CastToCharacter OtherActor))
  (Variables|Default|SetPlayer _ascharacter))

(event OnComponentEndOverlap(Box)
  (params (OverlappedComponent :type Primitive%20Component%20Object%20Reference) (OtherActor :type Actor%20Object%20Reference) (OtherComp :type Primitive%20Component%20Object%20Reference) (OtherBodyIndex :type Integer))
  (Variables|Default|SetInBox false))

(event EventBeginPlay)

(event Collision|EventActorBeginOverlap
  (params (OtherActor :type Actor%20Object%20Reference)))

(event EventTick
  (params (DeltaSeconds :type Float%20%28single-precision%29))
  (bind _player (Variables|Default|GetPlayer))
  (bind _otherend (Variables|Default|GetOtherEnd))
  (bind _player_2 (Variables|Default|GetPlayer))
  (bind _returnvalue (Transformation|GetActorLocation _otherend))
  (if (Variables|Default|GetInBox)
    (bind _asbp_standard_character (Utilities|Casting|CastToBP_StandardCharacter _player)
      (:then
        (if (Variables|/Game/Player/BP_StandardCharacter.BP_StandardCharacter_C|GetMoveUp _asbp_standard_character)
          (Utilities|IsValid _player_2
            (:Is%20Valid
              (Transformation|SetActorLocation _player_2 _returnvalue false true)
              (Variables|/Game/Player/BP_StandardCharacter.BP_StandardCharacter_C|SetMoveUp _asbp_standard_character false)))))
      (:CastFailed
        (bind _asbp_vrcharacter (Utilities|Casting|CastToBP_VRCharacter _player)
          (:then
            (if (Variables|/Game/Player/BP_VRCharacter.BP_VRCharacter_C|GetMoveUp _asbp_vrcharacter)
              (Utilities|IsValid _player_2
                (:Is%20Valid
                  (Transformation|SetActorLocation _player_2 _returnvalue false true)
                  (Variables|/Game/Player/BP_VRCharacter.BP_VRCharacter_C|SetMoveUp _asbp_vrcharacter false)))))
          (:CastFailed
            (Variables|Default|SetInBox false)))))))

(fn ConstructionScript)