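; Ladder actor that raises a standard or VR character standing in its trigger box while their MoveUp flag is set.
; Each Tick, MoveActorUp snaps the climber to the ladder's X/Y and adds a fixed, frame-rate-dependent Z step; leaving the box restores Walking.
; VRorStandard selects the character branch on overlap, but its fallback repeats the Standard cast, so it never sets SwitchPlayer false.
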(event OnComponentBeginOverlap(Box)
  (params (OverlappedComponent :type Primitive%20Component%20Object%20Reference) (OtherActor :type Actor%20Object%20Reference) (OtherComp :type Primitive%20Component%20Object%20Reference) (OtherBodyIndex :type Integer) (bFromSweep :type Boolean) (SweepResult :type Hit%20Result%20Structure%20%28by%20ref%29))
  (Variables|Default|SetInBox true)
  (Variables|Default|SetPlayer OtherActor)
  (CallFunction|VRorStandard OtherActor))

(event OnComponentEndOverlap(Box)
  (params (OverlappedComponent :type Primitive%20Component%20Object%20Reference) (OtherActor :type Actor%20Object%20Reference) (OtherComp :type Primitive%20Component%20Object%20Reference) (OtherBodyIndex :type Integer))
  (bind _player (Variables|Default|GetPlayer))
  (Variables|Default|SetInBox false)
  (if (Variables|Default|GetbSwitchPlayer)
    (bind _asbp_standard_character (Utilities|Casting|CastToBP_StandardCharacter _player))
    (Pawn|Components|CharacterMovement|SetMovementMode (Variables|/Script/Engine.Character|GetCharacterMovement _asbp_standard_character) "MOVE_Walking" 0)
    (else
      (bind _asbp_vrcharacter (Utilities|Casting|CastToBP_VRCharacter _player))
      (Pawn|Components|CharacterMovement|SetMovementMode (Variables|/Script/Engine.Character|GetCharacterMovement _asbp_vrcharacter) "MOVE_Walking" 0))))

(event EventBeginPlay)

(event Collision|EventActorBeginOverlap
  (params (OtherActor :type Actor%20Object%20Reference)))

(event EventTick
  (params (DeltaSeconds :type Float%20%28single-precision%29))
  (bind _player (Variables|Default|GetPlayer))
  (if (Variables|Default|GetInBox)
    (if (Variables|Default|GetbSwitchPlayer)
      (bind _asbp_standard_character (Utilities|Casting|CastToBP_StandardCharacter _player))
      (if (Variables|/Game/Player/BP_StandardCharacter.BP_StandardCharacter_C|GetMoveUp _asbp_standard_character)
        (Variables|/Game/Player/BP_StandardCharacter.BP_StandardCharacter_C|SetInBox _asbp_standard_character true)
        (CallFunction|MoveActorUp (Variables|Default|GetPlayer) :!label _label))
      (else
        (bind _asbp_vrcharacter (Utilities|Casting|CastToBP_VRCharacter _player))
        (Development|PrintString "VR")
        (if (Variables|/Game/Player/BP_VRCharacter.BP_VRCharacter_C|GetMoveUp _asbp_vrcharacter)
          (Variables|/Game/Player/BP_VRCharacter.BP_VRCharacter_C|SetInBox _asbp_vrcharacter true)
          (goto _label))))))

(fn ConstructionScript)

(fn VRorStandard
  (params (Actor :type Actor%20Object%20Reference))
  (Utilities|Casting|CastToBP_StandardCharacter Actor
    (:then
      (Variables|Default|SetbSwitchPlayer true))
    (:CastFailed
      (Utilities|Casting|CastToBP_StandardCharacter Actor)
      (Variables|Default|SetbSwitchPlayer false))))

(fn MoveActorUp
  (params (Actor :type Actor%20Object%20Reference))
  (bind _returnvalue (Transformation|GetActorLocation))
  (Transformation|SetActorLocation Actor (Math|Vector|MakeVector (.x _returnvalue) (.y _returnvalue) (+ (.z (Transformation|GetActorLocation Actor)) 2.0)) false false))