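; LadderTop is a trigger volume, apparently for the top of a ship's ladder, that carries an overlapping character along world Y.
; Box overlap stores the character and switches it to Flying; any end overlap restores that character to Walking.
; While occupied, Tick pins the character to the actor's X and Z, advancing Y by ShipRef's Speed plus a fixed offset each frame, without delta-time scaling.
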(event OnComponentBeginOverlap(Box)
  (params (OverlappedComponent :type Primitive%20Component%20Object%20Reference) (OtherActor :type Actor%20Object%20Reference) (OtherComp :type Primitive%20Component%20Object%20Reference) (OtherBodyIndex :type Integer) (bFromSweep :type Boolean) (SweepResult :type Hit%20Result%20Structure%20%28by%20ref%29))
  (bind _ascharacter (Utilities|Casting|CastToCharacter OtherActor))
  (Variables|Default|SetPlayer _ascharacter)
  (Variables|Default|SetInBox true)
  (Pawn|Components|CharacterMovement|SetMovementMode (Variables|/Script/Engine.Character|GetCharacterMovement _ascharacter) "MOVE_Flying" 0))

(event OnComponentEndOverlap(Box)
  (params (OverlappedComponent :type Primitive%20Component%20Object%20Reference) (OtherActor :type Actor%20Object%20Reference) (OtherComp :type Primitive%20Component%20Object%20Reference) (OtherBodyIndex :type Integer))
  (Variables|Default|SetInBox false)
  (bind _ascharacter (Utilities|Casting|CastToCharacter (Variables|Default|GetPlayer)))
  (Pawn|Components|CharacterMovement|SetMovementMode (Variables|/Script/Engine.Character|GetCharacterMovement _ascharacter) "MOVE_Walking" 0))

(event EventBeginPlay)

(event Collision|EventActorBeginOverlap
  (params (OtherActor :type Actor%20Object%20Reference)))

(event EventTick
  (params (DeltaSeconds :type Float%20%28single-precision%29))
  (bind _returnvalue (Transformation|GetActorLocation))
  (bind _player (Variables|Default|GetPlayer))
  (if (Variables|Default|GetInBox)
    (Transformation|SetActorLocation _player (Math|Vector|MakeVector (.x _returnvalue) (+ (+ (.y (Transformation|GetActorLocation _player)) (Variables|/Game/Models/Ship.Ship_C|GetSpeed (Variables|Default|GetShipRef))) 3.0) (.z _returnvalue)) false false)))

(fn ConstructionScript)