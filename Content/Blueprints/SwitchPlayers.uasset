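; SwitchPlayers is a Blueprint meant to switch a player between VR and standard characters, with events named for server execution.
; Two functions spawn the new character at the other's transform and destroy that one, falling back to PlayerStart if none exists.
; Toggle, spawn and possession logic, including HMD and stereo switching, is disconnected from its events, so none runs.
; Debug prints and authority checks trace the flow.
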(event Custom|SpawnPlayerServer_event
  (params (Switch%20Player :type Switch%20Players%20Object%20Reference) (Player%20Controller :type Player%20Controller%20Object%20Reference)))

(event Custom|Spawn%20Standard%20Player%20on%20Server
  (params (Switch%20Player :type Switch%20Players%20Object%20Reference) (Player%20Controller :type Player%20Controller%20Object%20Reference)))

(event Custom|Possess%20VR%20Player%20on%20Server
  (params (Player%20Controller :type Player%20Controller%20Object%20Reference) (Player%20to%20Possess :type BP%20VR%20Character%20Object%20Reference)))

(event Custom|Possess%20Standard%20Player%20on%20Server
  (params (Player%20Controller :type Player%20Controller%20Object%20Reference) (Player%20to%20Possess :type BP%20Standard%20Character%20Object%20Reference)))

(event Custom|Input)

(event EventBeginPlay)

(fn ConstructionScript)

(fn SpawnVRPlayer
  (params (Switch%20Player :type Switch%20Players%20Object%20Reference))
  (bind _standard_player (Variables|SwitchPlayers_C|GetStandard%20Player Switch%20Player))
  (Networking|SwitchHasAuthority
    (:Authority
      (Development|PrintString "Has authority" true true "(R=0.000000,G=0.660000,B=1.000000,A=1.000000)" 15.0))
    (:Remote
      (Development|PrintString "Does not have authority" true true "(R=0.000000,G=0.660000,B=1.000000,A=1.000000)" 15.0)))
  (Utilities|IsValid _standard_player
    (:Is%20Valid
      (Development|PrintString "Standard Player is valid" true true "(R=0.000000,G=0.660000,B=1.000000,A=1.000000)" 1e+01)
      (bind _returnvalue (Game|SpawnActorfromClass "/Game/Player/BP_VRCharacter.BP_VRCharacter_C" (Transformation|GetActorTransform _standard_player) "Undefined" 0 0))
      (Variables|SwitchPlayers_C|SetVR%20Player Switch%20Player _returnvalue)
      (Actor|DestroyActor (Variables|SwitchPlayers_C|GetStandard%20Player Switch%20Player)))
    (:Is%20Not%20Valid
      (Development|PrintString "Standard Player is NOT valid" true true "(R=0.000000,G=0.660000,B=1.000000,A=1.000000)" 1e+01)
      (bind _returnvalue_2 (Game|SpawnActorfromClass "/Game/Player/BP_VRCharacter.BP_VRCharacter_C" (Transformation|GetActorTransform (Variables|Default|GetPlayer%20Start)) "Undefined" 0 0))
      (Variables|SwitchPlayers_C|SetVR%20Player Switch%20Player _returnvalue_2)))
  (return (Variables|SwitchPlayers_C|GetVR%20Player Switch%20Player)))

(fn SpawnStandardPlayer
  (params (Switch%20Player :type Switch%20Players%20Object%20Reference))
  (bind _vr_player (Variables|SwitchPlayers_C|GetVR%20Player Switch%20Player))
  (Networking|SwitchHasAuthority
    (:Authority
      (Development|PrintString "Has authority" true true "(R=0.000000,G=0.660000,B=1.000000,A=1.000000)" 15.0))
    (:Remote
      (Development|PrintString "Does not have authority" true true "(R=0.000000,G=0.660000,B=1.000000,A=1.000000)" 15.0)))
  (Utilities|IsValid _vr_player
    (:Is%20Valid
      (Development|PrintString "VR Player is valid" true true "(R=0.000000,G=0.660000,B=1.000000,A=1.000000)" 1e+01)
      (bind _returnvalue (Game|SpawnActorfromClass "/Game/Player/BP_StandardCharacter.BP_StandardCharacter_C" (Transformation|GetActorTransform _vr_player) "Undefined" 0 0))
      (Variables|SwitchPlayers_C|SetStandard%20Player Switch%20Player _returnvalue)
      (Actor|DestroyActor (Variables|SwitchPlayers_C|GetVR%20Player Switch%20Player)))
    (:Is%20Not%20Valid
      (Development|PrintString "VR Player is NOT valid" true true "(R=0.000000,G=0.660000,B=1.000000,A=1.000000)" 1e+01)
      (bind _returnvalue_2 (Game|SpawnActorfromClass "/Game/Player/BP_StandardCharacter.BP_StandardCharacter_C" (Transformation|GetActorTransform (Variables|Default|GetPlayer%20Start)) "Undefined" 0 0))
      (Variables|SwitchPlayers_C|SetStandard%20Player Switch%20Player _returnvalue_2)))
  (return (Variables|SwitchPlayers_C|GetStandard%20Player Switch%20Player)))