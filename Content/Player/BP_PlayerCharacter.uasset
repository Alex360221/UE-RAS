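; VR player character that picks up and drops physics objects with either motion controller, using a floor tracking origin.
; Each grip press line-traces forward from that controller (with debug drawing), disables physics on a simulating hit and snaps its actor to that hand's hold point.
; Grip release detaches the actor and restores physics.
; EnableVR and DisableVR swap headset and first-person cameras, but their calls in the event graph are unwired.
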(event EventBeginPlay
  (Class|HeadMountedDisplayFunctionLibrary|SetTrackingOrigin "Floor"))

(event Collision|EventActorBeginOverlap
  (params (OtherActor :type Actor%20Object%20Reference)))

(event EventTick
  (params (DeltaSeconds :type Float%20%28single-precision%29)))

(event Input|ActionEvents|InputActionLeftGrip
  (params (Key :type Key%20Structure :default "None"))
  ;[1 1 1] Pickup and Drop
  (:Pressed
    (if (not (Variables|Default|GetIsHoldingObjectLeft))
      (CallFunction|LeftPickup)))
  (:Released
    (CallFunction|LeftDrop)))

(event Input|ActionEvents|InputActionRightGrip
  (params (Key :type Key%20Structure :default "None"))
  ;[1 1 1] Pickup and Drop
  (:Pressed
    (if (not (Variables|Default|GetIsHoldingObjectRight))
      (CallFunction|RightPickup)))
  (:Released
    (CallFunction|RightDrop)))

(fn ConstructionScript)

(fn LeftPickup
  (bind _mc_left (Variables|Default|GetMC_Left))
  (bind _returnvalue (Transformation|GetWorldLocation _mc_left))
  (bind (_outhit _returnvalue_2) (Collision|LineTraceForObjects _returnvalue (+ _returnvalue (* (Math|Vector|GetForwardVector _mc_left) 1e+02)) (Utilities|Array|MakeArray "ObjectTypeQuery4") false 0 "ForDuration"))
  (if _returnvalue_2
    (Variables|Default|SetLeft%20Hit%20Component (.HitComponent (Collision|BreakHitResult _outhit)))
    (if (Physics|IsSimulatingPhysics (Variables|Default|GetLeft%20Hit%20Component) "None")
      (bind _output_get (Variables|Default|SetLeftPickedUpActor (.HitActor (Collision|BreakHitResult _outhit))))
      (Physics|SetSimulatePhysics (Variables|Default|GetLeft%20Hit%20Component) false)
      (Transformation|AttachComponentToComponent _output_get (Variables|Default|GetLeftHeldObjLoc) "None" "SnapToTarget" "SnapToTarget" "KeepWorld" true)
      (Variables|Default|SetIsHoldingObjectLeft true))))

(fn RightPickup
  (bind _mc_right (Variables|Default|GetMC_Right))
  (bind _returnvalue (Transformation|GetWorldLocation _mc_right))
  (bind (_outhit _returnvalue_2) (Collision|LineTraceForObjects _returnvalue (+ _returnvalue (* (Math|Vector|GetForwardVector _mc_right) 1e+02)) (Utilities|Array|MakeArray "ObjectTypeQuery4") false 0 "ForDuration"))
  (if _returnvalue_2
    (Variables|Default|SetRight%20Hit%20Component (.HitComponent (Collision|BreakHitResult _outhit)))
    (if (Physics|IsSimulatingPhysics (Variables|Default|GetRight%20Hit%20Component) "None")
      (bind _output_get (Variables|Default|SetRightPickedUpActor (.HitActor (Collision|BreakHitResult _outhit))))
      (Physics|SetSimulatePhysics (Variables|Default|GetRight%20Hit%20Component) false)
      (Transformation|AttachComponentToComponent _output_get (Variables|Default|GetRightHeldObjLoc) "None" "SnapToTarget" "SnapToTarget" "KeepWorld" true)
      (Variables|Default|SetIsHoldingObjectRight true))))

(fn LeftDrop
  (Utilities|IsValid (Variables|Default|GetLeftPickedUpActor)
    (:Is%20Valid
      (Transformation|DetachFromActor (Variables|Default|GetLeftPickedUpActor) "KeepWorld" "KeepWorld" "KeepWorld")
      (Utilities|IsValid (Variables|Default|GetLeft%20Hit%20Component)
        (:Is%20Valid
          (Physics|SetSimulatePhysics (Variables|Default|GetLeft%20Hit%20Component) true)
          (Variables|Default|SetIsHoldingObjectLeft false)
          (Variables|Default|SetLeft%20Hit%20Component 0)
          (Variables|Default|SetLeftPickedUpActor 0))))))

(fn RightDrop
  (Utilities|IsValid (Variables|Default|GetRightPickedUpActor)
    (:Is%20Valid
      (Transformation|DetachFromActor (Variables|Default|GetRightPickedUpActor) "KeepWorld" "KeepWorld" "KeepWorld")
      (Utilities|IsValid (Variables|Default|GetRight%20Hit%20Component)
        (:Is%20Valid
          (Physics|SetSimulatePhysics (Variables|Default|GetRight%20Hit%20Component) true)
          (Variables|Default|SetIsHoldingObjectRight false)
          (Variables|Default|SetRight%20Hit%20Component 0)
          (Variables|Default|SetRightPickedUpActor 0))))))

(fn EnableVR
  (if (not (Class|HeadMountedDisplayFunctionLibrary|IsHeadMountedDisplayEnabled))
    (Class|HeadMountedDisplayFunctionLibrary|EnableHMD true)
    (Components|Activation|SetActive (Variables|Default|GetVRCameraComp) true false)
    (Components|Activation|SetActive (Variables|Default|GetFPCameraComp) false false)
    (Rendering|SetVisibility (Variables|Default|GetMC_Left) true true)))

(fn DisableVR
  (bind _fpcameracomp (Variables|Default|GetFPCameraComp))
  (if (Class|HeadMountedDisplayFunctionLibrary|IsHeadMountedDisplayEnabled)
    (Class|HeadMountedDisplayFunctionLibrary|EnableHMD false)
    (Components|Activation|SetActive _fpcameracomp true false)
    (Components|Activation|SetActive (Variables|Default|GetVRCameraComp) false false)
    (Rendering|SetVisibility (Variables|Default|GetMC_Left) false true)
    (Development|PrintString (Utilities|String|ToString(Rotator) (Variables|/Script/Engine.SceneComponent|GetRelativeRotation _fpcameracomp)))))