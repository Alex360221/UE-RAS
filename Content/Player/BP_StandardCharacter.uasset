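; BP_StandardCharacter is the non-VR player character, which can swap itself for BP_VRCharacter at runtime.
; On BeginPlay it adds a crosshair and caches the ship, storing the respawn point and map controller in the game instance.
; Inputs toggle the pause menu, set a MoveUp flag from Teleport, or destroy this pawn and possess a new VR character with stereo enabled.
; The flying-mode ladder climb logic is disconnected and never runs.
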(event EventBeginPlay
  ;[1 1 1] Variable Setting
  (CallFunction|CreateHUD)
  (bind _outactors (Actor|GetAllActorsOfClass "/Game/Models/Ship.Ship_C"))
  (Variables|Default|SetShipRef (Utilities|Array|Get(acopy) _outactors))
  (bind _ascustom_game_instance (Utilities|Casting|CastToCustomGameInstance (Game|GetGameInstance)))
  (bind _outactors_2 (Actor|GetAllActorswithTag "RespawnPoint"))
  (Variables|/Script/RAS_Trainer.CustomGameInstance|SetRespawnPoint _ascustom_game_instance (Utilities|Array|Get(acopy) _outactors_2))
  (bind _outactors_3 (Actor|GetAllActorsOfClass "/Script/RAS_Trainer.MapController"))
  (bind _ascustom_game_instance_2 (Utilities|Casting|CastToCustomGameInstance (Game|GetGameInstance)))
  (Variables|/Script/RAS_Trainer.CustomGameInstance|SetMapController _ascustom_game_instance_2 (Utilities|Array|Get(acopy) _outactors_3)))

(event EventTick
  (params (DeltaSeconds :type Float%20%28single-precision%29))
  ;[1 1 1] Ladder
)

(event Input|ActionEvents|InputActionSwitchCharacter
  (params (Key :type Key%20Structure :default "None"))
  ;[1 1 1] Switch to VR Character
  (:Pressed
    (Variables|Default|SetSwapPoint (Transformation|GetWorldTransform (Variables|Default|GetCapsuleComponent)))
    (Pawn|UnPossess (Game|GetPlayerController 0))
    (Actor|DestroyActor)
    (bind _returnvalue (Game|SpawnActorfromClass "/Game/Player/BP_VRCharacter.BP_VRCharacter_C" (Variables|Default|GetSwapPoint) "Undefined" 0 0))
    (Class|HeadMountedDisplayFunctionLibrary|EnableHMD true)
    (Development|ExecuteConsoleCommand "vr.bEnableStereo 1" 0)
    (Class|HeadMountedDisplayFunctionLibrary|SetTrackingOrigin "Floor")
    (Pawn|Possess (Game|GetPlayerController 0) _returnvalue)))

(event Input|ActionEvents|InputActionPauseMenu
  (params (Key :type Key%20Structure :default "None"))
  (bind _returnvalue (Game|GetPlayerController 0))
  ;[1 1 1] Pause / Unpause
  (:Pressed
    (Utilities|IsValid (Variables|Default|GetPM_REF)
      (:Is%20Valid
        _)
      (:Is%20Not%20Valid
        (bind _returnvalue_2 (UserInterface|CreateWidget "/Game/UI/PauseMenu.PauseMenu_C"))
        (Variables|Default|SetPM_REF _returnvalue_2)))
    (if (Game|IsGamePaused)
      (Widget|RemovefromParent (Variables|Default|GetPM_REF))
      (Game|SetGamePaused false)
      (Variables|/Script/Engine.PlayerController|SetbShowMouseCursor _returnvalue false)
      (Input|SetInputModeGameOnly _returnvalue)
      (else
        (UserInterface|Viewport|AddtoViewport (Variables|Default|GetPM_REF) 0)
        (Game|SetGamePaused true)
        (Variables|/Script/Engine.PlayerController|SetbShowMouseCursor _returnvalue true)
        (Input|SetInputModeGameandUI _returnvalue (Variables|Default|GetPM_REF) "LockInFullscreen" false)))))

(event Input|ActionEvents|InputActionTeleport
  (params (Key :type Key%20Structure :default "None"))
  ;[1 1 1] Teleport
  (:Pressed
    (Variables|Default|SetMoveUp true))
  (:Released
    (Variables|Default|SetMoveUp false)))

(event Input|KeyboardEvents|E
  (params (Key :type Key%20Structure :default "None"))
  ;[1 1 1] Ladder
)

(fn ConstructionScript)

(fn CreateHUD
  (bind _returnvalue (UserInterface|CreateWidget "/Game/UI/Crosshair.Crosshair_C"))
  (UserInterface|Viewport|AddtoViewport _returnvalue 0))