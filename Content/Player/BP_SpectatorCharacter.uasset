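; BP_SpectatorCharacter is a player character that can toggle a pause menu and switch back to the standard character.
; Switching destroys it, spawns BP_StandardCharacter at its capsule transform, disables HMD and stereo rendering, then possesses the new character.
; While not walking, Tick drifts the capsule along the ship's direction and speed read from CustomGameInstance.
; BeginPlay stores the first RespawnPoint-tagged actor in that game instance.
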(event EventBeginPlay
  ;[1 1 1] Set respawn point
  (bind _ascustom_game_instance (Utilities|Casting|CastToCustomGameInstance (Game|GetGameInstance)))
  (bind _outactors (Actor|GetAllActorswithTag "RespawnPoint"))
  (Variables|/Script/RAS_Trainer.CustomGameInstance|SetRespawnPoint _ascustom_game_instance (Utilities|Array|Get(acopy) _outactors)))

(event EventTick
  (params (DeltaSeconds :type Float%20%28single-precision%29))
  (bind _capsulecomponent (Variables|Default|GetCapsuleComponent))
  (bind _returnvalue (Transformation|GetWorldTransform _capsulecomponent))
  (bind (_location _rotation _scale) (Math|Transform|BreakTransform _returnvalue))
  ;[1 1 1] Moves spectator character with the speed & direction of the ship when flying
  (if (not (Pawn|Components|CharacterMovement|IsWalking (Variables|Character|GetCharacterMovement)))
    (bind _ascustom_game_instance (Utilities|Casting|CastToCustomGameInstance (Game|GetGameInstance)))
    (Variables|Default|SetDirection (Variables|/Script/RAS_Trainer.CustomGameInstance|GetShipDirection _ascustom_game_instance))
    (Variables|Default|SetSpeed (Variables|/Script/RAS_Trainer.CustomGameInstance|GetShipSpeed _ascustom_game_instance))
    (Transformation|SetWorldTransform (Variables|Default|GetCapsuleComponent) (Math|Transform|MakeTransform (+ (* (Math|Vector|Normalize (Variables|Default|GetDirection)) (* (Utilities|Time|GetWorldDeltaSeconds) (Variables|Default|GetSpeed))) _location) _rotation _scale) false false)))

(event Input|ActionEvents|InputActionSwitchCharacter
  (params (Key :type Key%20Structure :default "None"))
  ;[1 1 1] Switch to Standard Character
  (:Pressed
    (Variables|Default|SetSwapPoint (Transformation|GetWorldTransform (Variables|Default|GetCapsuleComponent)))
    (Pawn|UnPossess (Game|GetPlayerController 0))
    (Actor|DestroyActor)
    (bind _returnvalue (Game|SpawnActorfromClass "/Game/Player/BP_StandardCharacter.BP_StandardCharacter_C" (Variables|Default|GetSwapPoint) "Undefined" 0 0))
    (Class|HeadMountedDisplayFunctionLibrary|EnableHMD false)
    (Development|ExecuteConsoleCommand "vr.bEnableStereo 0" 0)
    (Pawn|Possess (Game|GetPlayerController 0) _returnvalue)))

(event Input|ActionEvents|InputActionPauseMenu
  (params (Key :type Key%20Structure :default "None"))
  (bind _returnvalue (Game|GetPlayerController 0))
  ;[1 1 1] Pause / Unpause
  (:Pressed
    (Utilities|IsValid (Variables|Default|GetPM_REF)
      (:Is%20Valid
        _)
      (:Is%20Not%20Valid
        (bind _returnvalue_2 (UserInterface|CreateWidget "/Game/UI/PauseMenu.PauseMenu_C"))
        (Variables|Default|SetPM_REF _returnvalue_2)))
    (if (Game|IsGamePaused)
      (Widget|RemovefromParent (Variables|Default|GetPM_REF))
      (Game|SetGamePaused false)
      (Variables|/Script/Engine.PlayerController|SetbShowMouseCursor _returnvalue false)
      (Input|SetInputModeGameOnly _returnvalue)
      (else
        (UserInterface|Viewport|AddtoViewport (Variables|Default|GetPM_REF) 0)
        (Game|SetGamePaused true)
        (Variables|/Script/Engine.PlayerController|SetbShowMouseCursor _returnvalue true)
        (Input|SetInputModeGameandUI _returnvalue (Variables|Default|GetPM_REF) "LockInFullscreen" false)))))

(fn ConstructionScript)